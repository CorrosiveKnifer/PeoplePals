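; Door Blueprint that swings a door component between closed and open when Interact is called.
; Interact only flips the IsOpen flag.
; Tick moves the door's relative rotation toward zero or the OpenRotation yaw with a shortest-path lerp.
; The fixed alpha applied every frame gives an eased motion whose speed depends on frame rate.
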(event `self.ReceiveTick`
  (params (DeltaSeconds :type "Float (single-precision)"))
  (bind _door (`self.Door`))
  (if (not (`self.IsOpen`))
    (`SceneComponent.K2_SetRelativeRotation` _door (`KismetMathLibrary.RLerp` (`SceneComponent.RelativeRotation` _door) (struct) 0.05 true) false false)
    (else
      (`SceneComponent.K2_SetRelativeRotation` _door (`KismetMathLibrary.RLerp` (`SceneComponent.RelativeRotation` _door) (`KismetMathLibrary.MakeRotator` 0.0 0.0 (`self.OpenRotation`)) 0.05 true) false false))))

(fn `Interact`
  (set `self.IsOpen` (not (`self.IsOpen`))))

(fn `UserConstructionScript`)