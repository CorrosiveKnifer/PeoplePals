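; Parent Blueprint for sprite-based tank parts that snap together on a 2D grid, forming a graph of North/South/East/West neighbour links around a core at (0,0).
; Add functions link new parts to neighbours and attach them to sprite sockets, remapping socket names to the parent's rotation.
; Recursive "BFS" searches gather connected parts.
; Removal unlinks a part, re-sockets neighbours and recursively removes any stranded ones, optionally spawning Paper_Drop pickups.
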(event `self.ReceiveBeginPlay`)

(fn `AddExistingToPos`
  (params (Position :type "Vector2D Structure") (`New Part` :type "/Game/Tank/Blueprints/Parents/Paper_Part Object Reference"))
  (returns (Added :type Boolean))
  (bind _position (`self.Position`))
  (if (`KismetMathLibrary.EqualExactly_Vector2DVector2D` Position (+ _position (0.0 -1.0)))
    (bind _added (`self.AddExistingToSlot` self "South" `New Part` true))
    (bind _asbase_player (cast `/Game/Player/BasePlayer` (`GameplayStatics.GetPlayerPawn` 0)))
    (`/Game/Player/BasePlayer.Refresh` _asbase_player)
    (return _added)
    (elif (`KismetMathLibrary.EqualExactly_Vector2DVector2D` Position (+ _position (0.0 1.0)))
      (bind _added_2 (`self.AddExistingToSlot` self "North" `New Part` true))
      (bind _asbase_player_2 (cast `/Game/Player/BasePlayer` (`GameplayStatics.GetPlayerPawn` 0)))
      (`/Game/Player/BasePlayer.Refresh` _asbase_player_2)
      (return _added_2)
      (elif (`KismetMathLibrary.EqualExactly_Vector2DVector2D` Position (+ _position (-1.0 0.0)))
        (bind _added_3 (`self.AddExistingToSlot` self "West" `New Part` true))
        (bind _asbase_player_3 (cast `/Game/Player/BasePlayer` (`GameplayStatics.GetPlayerPawn` 0)))
        (`/Game/Player/BasePlayer.Refresh` _asbase_player_3)
        (return _added_3)
        (elif (`KismetMathLibrary.EqualExactly_Vector2DVector2D` Position (+ _position (1.0 0.0)))
          (bind _added_4 (`self.AddExistingToSlot` self "East" `New Part` true))
          (bind _asbase_player_4 (cast `/Game/Player/BasePlayer` (`GameplayStatics.GetPlayerPawn` 0)))
          (`/Game/Player/BasePlayer.Refresh` _asbase_player_4)
          (return _added_4)
          (else
            (return false)))))))

(fn `AddExistingToSlot`
  (params (Loc :type Name) (`Existing Part` :type "/Game/Tank/Blueprints/Parents/Paper_Part Object Reference") (Socket :type Boolean :default true))
  (returns (Added :type Boolean))
  (bind _position (`self.Position`))
  (`/Engine/EditorBlueprintResources/StandardMacros.IsValid` (`PaperSpriteComponent.GetSprite` (`self.RenderComponent`))
    (:`Is Valid`
      (if (`KismetArrayLibrary.Array_Contains` (`SceneComponent.GetAllSocketNames` (`self.RenderComponent`)) Loc)
        (if (and (== Loc "South") (not (`KismetSystemLibrary.IsValid` (`self.Part_South`))))
          (bind _output_get (set `self.Part_South` `Existing Part`))
          (set `/Game/Tank/Blueprints/Parents/Paper_Part.Position` (+ _position (0.0 -1.0)) _output_get)
          (`self.LinkToMap` _output_get self)
          (if Socket :!label _label
            (bind _socketed (`self.SocketPart` Loc `Existing Part`)))
          (return _socketed)
          (elif (and (== Loc "North") (not (`KismetSystemLibrary.IsValid` (`self.Part_North`))))
            (bind _output_get_2 (set `self.Part_North` `Existing Part`))
            (set `/Game/Tank/Blueprints/Parents/Paper_Part.Position` (+ _position (0.0 1.0)) _output_get_2)
            (`self.LinkToMap` _output_get_2 self)
            (goto _label)
            (elif (and (== Loc "West") (not (`KismetSystemLibrary.IsValid` (`self.Part_West`))))
              (bind _output_get_3 (set `self.Part_West` `Existing Part`))
              (set `/Game/Tank/Blueprints/Parents/Paper_Part.Position` (+ _position (-1.0 0.0)) _output_get_3)
              (`self.LinkToMap` _output_get_3 self)
              (goto _label)
              (elif (and (== Loc "East") (not (`KismetSystemLibrary.IsValid` (`self.Part_East`))))
                (bind _output_get_4 (set `self.Part_East` `Existing Part`))
                (set `/Game/Tank/Blueprints/Parents/Paper_Part.Position` (+ _position (1.0 0.0)) _output_get_4)
                (`self.LinkToMap` _output_get_4 self)
                (goto _label)
                (else
                  _)))))))
    (:`Is Not Valid`
      _))
  (return false))

(fn `AddNewToPos`
  (params (`New Part Class` :type "/Game/Tank/Blueprints/Parents/Paper_Part Class Reference") (Position :type "Vector2D Structure"))
  (returns (`Part Added` :type Boolean) (`New Part` :type "/Game/Tank/Blueprints/Parents/Paper_Part Object Reference"))
  (locals (`Array Of Possible Additions` :type "Array of /Game/Tank/Blueprints/Parents/Paper_Part Object Reference") (HasPartAdded :type Boolean))
  (bind _array_of_possible_additions (`local.Array Of Possible Additions`))
  (bind _haspartadded (`local.HasPartAdded`))
  (bind _returnvalue (`|SpawnActorFromClass` `New Part Class` (`KismetMathLibrary.MakeTransform` (0.0 0.0 0.0)) "AlwaysSpawn" "OverrideRootScale" null null))
  (bind _array (`self.BFS_GetAllParts` (`|MakeArray` self :!type "/Game/Tank/Blueprints/Parents/Paper_Part Object Reference")))
  (for _array_element _array
    (if (`KismetMathLibrary.EqualExactly_Vector2DVector2D` (`/Game/Tank/Blueprints/Parents/Paper_Part.Position` _array_element) Position)
      (`self.K2_DestroyActor` _returnvalue)
      (return false null)
      (else
        (bind _position (`/Game/Tank/Blueprints/Parents/Paper_Part.Position` _array_element))
        (if (or (`KismetMathLibrary.EqualExactly_Vector2DVector2D` _position (+ Position (0.0 -1.0))) (`KismetMathLibrary.EqualExactly_Vector2DVector2D` _position (+ Position (0.0 1.0))) (`KismetMathLibrary.EqualExactly_Vector2DVector2D` _position (+ Position (-1.0 0.0))) (`KismetMathLibrary.EqualExactly_Vector2DVector2D` _position (+ Position (1.0 0.0))))
          (`KismetArrayLibrary.Array_Add` _array_of_possible_additions _array_element)))))
  (for _array_element_2 _array_of_possible_additions
    (bind _added (`self.AddExistingToPos` _array_element_2 Position _returnvalue))
    (bind _output_get (set `local.HasPartAdded` _added))
    (if _output_get
      (break)))
  (if _haspartadded
    (return _haspartadded _returnvalue)
    (else
      (`self.K2_DestroyActor`)
      (return false null))))

(fn `AddNewToSlot`
  (params (Loc :type Name) (Part :type "/Game/Tank/Blueprints/Parents/Paper_Part Class Reference"))
  (returns (Added :type Boolean))
  (bind _returnvalue (`|SpawnActorFromClass` Part (`KismetMathLibrary.MakeTransform` (0.0 0.0 0.0)) "AlwaysSpawn" "OverrideRootScale" null null))
  (bind _added (`self.AddExistingToSlot` Loc _returnvalue))
  (if _added
    (return true)
    (else
      (`self.K2_DestroyActor` _returnvalue)
      (return false))))

(fn `BFS_ DoesPosExist`
  (params (Position :type "Vector2D Structure"))
  (returns (`Part Exist` :type Boolean) (`Part Ref` :type "/Game/Tank/Blueprints/Parents/Paper_Part Object Reference"))
  (bind _array (`self.BFS_GetAllParts` (`|MakeArray` self :!type "/Game/Tank/Blueprints/Parents/Paper_Part Object Reference")))
  (for _array_element _array
    (bind _returnvalue (`KismetMathLibrary.EqualExactly_Vector2DVector2D` Position (`/Game/Tank/Blueprints/Parents/Paper_Part.Position` _array_element)))
    (if _returnvalue
      (return _returnvalue _array_element)))
  (return false null))

(fn `BFS_GetAllParts`
  (params (`Part Array` :type "Array of /Game/Tank/Blueprints/Parents/Paper_Part Object Reference"))
  (returns (Array :type "Array of /Game/Tank/Blueprints/Parents/Paper_Part Object Reference"))
  (bind _array (`self.PartArray` (`self.Part_South`) `Part Array`))
  (bind _array_2 (`self.PartArray` (`self.Part_North`) _array))
  (bind _array_3 (`self.PartArray` (`self.Part_West`) _array_2))
  (bind _array_4 (`self.PartArray` (`self.Part_East`) _array_3))
  (return _array_4))

(fn `BFS_GetAllPartsOf`
  (params (`Class Of` :type "/Game/Tank/Blueprints/Parents/Paper_Part Class Reference"))
  (returns (`List of Parts` :type "Array of /Game/Tank/Blueprints/Parents/Paper_Part Object Reference"))
  (locals (`New Array` :type "Array of /Game/Tank/Blueprints/Parents/Paper_Part Object Reference"))
  (bind _new_array (`local.New Array`))
  (bind _array (`self.BFS_GetAllParts` (`|MakeArray` self :!type "/Game/Tank/Blueprints/Parents/Paper_Part Object Reference")))
  (for _array_element _array
    (if (== `Class Of` (`GameplayStatics.GetObjectClass` _array_element))
      (`KismetArrayLibrary.Array_Add` _new_array _array_element)))
  (return _new_array))

(fn `Get Location Name`
  (params (Part :type "/Game/Tank/Blueprints/Parents/Paper_Part Object Reference"))
  (returns (Loc :type Name))
  (locals (`Link in` :type "Array of /Game/Tank/Blueprints/Parents/Paper_Part Object Reference"))
  (bind _output_get (set `local.Link in` (`|MakeArray` (`self.Part_South`) (`self.Part_North`) (`self.Part_West`) (`self.Part_East`))))
  (for (_array_element _array_index) _output_get
    (if (== _array_element Part)
      (switch `int` _array_index
        (:`0`
          (return "South"))
        (:`1`
          (return "North"))
        (:`2`
          (return "West"))
        (:`3`
          (return "East")))))
  (return "None"))

(fn `GetArrayOfNonLinks`
  (returns (Array :type "Array of Vector2D Structure"))
  (locals (`Possible Pos` :type "Array of Vector2D Structure"))
  (bind _possible_pos (`local.Possible Pos`))
  (bind _position (`self.Position`))
  (bind _possible_pos_2 (`local.Possible Pos`))
  (bind _returnvalue (`SceneComponent.GetAllSocketNames` (`self.RenderComponent`)))
  (bind _returnvalue_2 (+ _position (0.0 -1.0)))
  (bind _returnvalue_3 (+ _position (0.0 1.0)))
  (bind _returnvalue_4 (+ _position (-1.0 0.0)))
  (bind _returnvalue_5 (+ _position (1.0 0.0)))
  (`KismetArrayLibrary.Array_Add` _possible_pos_2 _returnvalue_2)
  (`KismetArrayLibrary.Array_Add` _possible_pos_2 _returnvalue_3)
  (`KismetArrayLibrary.Array_Add` _possible_pos_2 _returnvalue_4)
  (`KismetArrayLibrary.Array_Add` _possible_pos_2 _returnvalue_5)
  (if (or (`KismetSystemLibrary.IsValid` (`self.Part_South`)) (not (`KismetArrayLibrary.Array_Contains` _returnvalue "South")))
    (`KismetArrayLibrary.Array_RemoveItem` _possible_pos _returnvalue_2))
  (if (or (`KismetSystemLibrary.IsValid` (`self.Part_North`)) (not (`KismetArrayLibrary.Array_Contains` _returnvalue "North")))
    (`KismetArrayLibrary.Array_RemoveItem` _possible_pos _returnvalue_3))
  (if (or (`KismetSystemLibrary.IsValid` (`self.Part_West`)) (not (`KismetArrayLibrary.Array_Contains` _returnvalue "West")))
    (`KismetArrayLibrary.Array_RemoveItem` _possible_pos _returnvalue_4))
  (if (or (`KismetSystemLibrary.IsValid` (`self.Part_East`)) (not (`KismetArrayLibrary.Array_Contains` _returnvalue "East")))
    (`KismetArrayLibrary.Array_RemoveItem` _possible_pos _returnvalue_5))
  (return (`local.Possible Pos`)))

(fn `InvertSocketName`
  (params (Name :type Name))
  (returns (Inverse :type Name))
  (switch `name` Name
    (:`South`
      (return "North"))
    (:`North`
      (return "South"))
    (:`West`
      (return "East"))
    (:`East`
      (return "West"))))

(fn `LinkToMap`
  (params (Core :type "/Game/Tank/Blueprints/Parents/Paper_Part Object Reference"))
  (bind _position (`self.Position`))
  (bind _array (`self.BFS_GetAllParts` Core (`|MakeArray` Core)))
  (for _array_element _array
    (if (`KismetMathLibrary.EqualExactly_Vector2DVector2D` (`/Game/Tank/Blueprints/Parents/Paper_Part.Position` _array_element) (+ _position (0.0 -1.0)))
      (bind _output_get (set `self.Part_South` _array_element))
      (set `/Game/Tank/Blueprints/Parents/Paper_Part.Part_North` self _output_get) ; Link back
      (elif (`KismetMathLibrary.EqualExactly_Vector2DVector2D` (`/Game/Tank/Blueprints/Parents/Paper_Part.Position` _array_element) (+ _position (0.0 1.0)))
        (bind _output_get_2 (set `self.Part_North` _array_element))
        (set `/Game/Tank/Blueprints/Parents/Paper_Part.Part_South` self _output_get_2) ; Link back
        (elif (`KismetMathLibrary.EqualExactly_Vector2DVector2D` (`/Game/Tank/Blueprints/Parents/Paper_Part.Position` _array_element) (+ _position (-1.0 0.0)))
          (bind _output_get_3 (set `self.Part_West` _array_element))
          (set `/Game/Tank/Blueprints/Parents/Paper_Part.Part_East` self _output_get_3) ; Link back
          (elif (`KismetMathLibrary.EqualExactly_Vector2DVector2D` (`/Game/Tank/Blueprints/Parents/Paper_Part.Position` _array_element) (+ _position (1.0 0.0)))
            (bind _output_get_4 (set `self.Part_East` _array_element))
            (set `/Game/Tank/Blueprints/Parents/Paper_Part.Part_West` self _output_get_4) ; Link back
          )))))
  (return))

(fn `Merge Array`
  (params (`Array A` :type "Array of /Game/Tank/Blueprints/Parents/Paper_Part Object Reference") (`Array B` :type "Array of /Game/Tank/Blueprints/Parents/Paper_Part Object Reference"))
  (returns (`Array C` :type "Array of /Game/Tank/Blueprints/Parents/Paper_Part Object Reference"))
  (for _array_element `Array A`
    (`KismetArrayLibrary.Array_AddUnique` `Array B` _array_element))
  (return `Array B`))

(fn `PartArray`
  (params (Part :type "/Game/Tank/Blueprints/Parents/Paper_Part Object Reference") (Array1 :type "Array of /Game/Tank/Blueprints/Parents/Paper_Part Object Reference (by ref)"))
  (returns (Array :type "Array of /Game/Tank/Blueprints/Parents/Paper_Part Object Reference (by ref)"))
  (`/Engine/EditorBlueprintResources/StandardMacros.IsValid` Part ; Does the part Exist?
    (:`Is Valid`
      (if (== (`KismetArrayLibrary.Array_Find` Array1 Part) -1)
        (`KismetArrayLibrary.Array_AddUnique` Array1 Part) ; Then, Add the node to the list
        (bind _array (`self.BFS_GetAllParts` Part Array1)) ; Expand List with linking parts
        (return _array)
        (else
          _)))
    (:`Is Not Valid`
      _))
  (return Array1) ; else, The part has already been added to the list OR it doesn't exist.
)

(fn `Remove Link`
  (params (`Link in` :type "/Game/Tank/Blueprints/Parents/Paper_Part Object Reference"))
  (locals (`Links out` :type "Array of /Game/Tank/Blueprints/Parents/Paper_Part Object Reference"))
  (bind _output_get (set `local.Links out` (`|MakeArray` (`self.Part_South`) (`self.Part_North`) (`self.Part_West`) (`self.Part_East`))))
  (for (_array_element _array_index) _output_get
    ;[1 1 1] Removes only the one that matches the link in.
    (if (and (== _array_element `Link in`) (`KismetSystemLibrary.IsValid` _array_element))
      (switch `int` _array_index
        (:`0`
          (set `self.Part_South` null))
        (:`1`
          (set `self.Part_North` null))
        (:`2`
          (set `self.Part_West` null))
        (:`3`
          (set `self.Part_East` null)))
      (return)))
  (return))

(fn `RemoveAtPos`
  (params (Pos :type "Vector2D Structure") (IsDropped :type Boolean) (IsExtrasDropped :type Boolean))
  (returns (`Part Exist` :type Boolean))
  (locals (`Links in` :type "Array of /Game/Tank/Blueprints/Parents/Paper_Part Object Reference") (Target :type "/Game/Tank/Blueprints/Parents/Paper_Part Object Reference"))
  (bind _target (`local.Target`))
  (bind _target_2 (`local.Target`))
  (bind _links_in (`local.Links in`))
  (bind _returnvalue_location (`KismetMathLibrary.BreakTransform` (`self.GetTransform` _target_2)))
  (if (`KismetMathLibrary.EqualExactly_Vector2DVector2D` Pos (`self.Position`))
    ;[1 1 1] If the position to be removed is itself
    (set `local.Target` self)
    (set `local.Links in` (`|MakeArray` (`self.Part_South`) (`self.Part_North`) (`self.Part_West`) (`self.Part_East`))) ; Keep a list of all links into other parts.
    (else
      ;[1 1 1] If position to be removed is linked (in some way).
      (bind (_part_exist _part_ref) (`self.BFS_ DoesPosExist` Pos))
      (if _part_exist
        (set `local.Target` _part_ref)
        (set `local.Links in` (`|MakeArray` (`/Game/Tank/Blueprints/Parents/Paper_Part.Part_South` _part_ref) (`/Game/Tank/Blueprints/Parents/Paper_Part.Part_North` _part_ref) (`/Game/Tank/Blueprints/Parents/Paper_Part.Part_West` _part_ref) (`/Game/Tank/Blueprints/Parents/Paper_Part.Part_East` _part_ref))) ; Keep a list of all links into other parts.
        (else
          (return _part_exist) ; Position never existed in the first place.
        ))))
  (`KismetArrayLibrary.Array_RemoveItem` _links_in) ; Remove Null items
  (for _array_element _links_in
    (`self.Remove Link` _array_element (`local.Target`)) ; Remove the link back to this part.
  )
  (for _array_element_2 (`local.Links in`)
    (if (`KismetMathLibrary.NotEqualExactly_Vector2DVector2D` (`/Game/Tank/Blueprints/Parents/Paper_Part.Position` _array_element_2))
      (bind _part_exist_2 (`self.BFS_ DoesPosExist` _array_element_2 (0.0 0.0))) ; Check if each link still links towards the core.
      (if _part_exist_2
        (bind _could_relink (`self.ReSocket` _array_element_2))
        (if (not _could_relink)
          (`self.RemoveAtPos` _array_element_2 (`/Game/Tank/Blueprints/Parents/Paper_Part.Position` _array_element_2) IsExtrasDropped IsExtrasDropped :!label _label) ; Is No longer reachable
        )
        (else
          (goto _label)))))
  (if IsDropped
    ;[1 1 1] Spawn Paper_Drop
    (bind _returnvalue (`|SpawnActorFromClass` "/Game/Tank/Blueprints/Paper_Drop.Paper_Drop_C" (`KismetMathLibrary.MakeTransform` _returnvalue_location) "AlwaysSpawn" "OverrideRootScale" null null))
    ;[1 1 1] Set up the drop.
    (`PaperSpriteComponent.SetSprite` (`PaperSpriteActor.RenderComponent` _returnvalue) (`PaperSpriteComponent.GetSprite` (`PaperSpriteActor.RenderComponent` _target)))
    (set `/Game/Tank/Blueprints/Paper_Drop.Part Class` (`GameplayStatics.GetObjectClass` _target) _returnvalue)
    ;[1 1 1] Destroy the part
    (`self.K2_DestroyActor` _target)
    (return true) ; Drop
    (else
      ;[1 1 1] Destroy the part
      (`self.K2_DestroyActor` _target_2)
      (return true) ; Destroy
    )))

(fn `ReSocket`
  (returns (`Could Relink` :type Boolean))
  (locals (`Links in` :type "Array of /Game/Tank/Blueprints/Parents/Paper_Part Object Reference"))
  (bind _links_in (`local.Links in`))
  (bind _inverse (`self.InvertSocketName` (`self.SocketLoc`)))
  (bind _output_get (set `local.Links in` (`|MakeArray` (`self.Part_South`) (`self.Part_North`) (`self.Part_West`) (`self.Part_East`))))
  ;[1 1 1] Remove previous socket from the list.
  (switch `name` _inverse
    (:`South`
      (`KismetArrayLibrary.Array_Remove` _output_get))
    (:`North`
      (`KismetArrayLibrary.Array_Remove` _output_get 1))
    (:`West`
      (`KismetArrayLibrary.Array_Remove` _output_get 2))
    (:`East`
      (`KismetArrayLibrary.Array_Remove` _output_get 3)))
  ;[1 1 1] Check if the link in, is socketed to this part.
  (`KismetArrayLibrary.Array_RemoveItem` _links_in) ; Remove Null
  (for _array_element _links_in
    (`/Engine/EditorBlueprintResources/StandardMacros.IsValid` _array_element
      (:`Is Valid`
        (bind _loc (`self.Get Location Name` _array_element))
        (bind _inverse_2 (`self.InvertSocketName` _loc)) ; Link out name
        (if (== (`/Game/Tank/Blueprints/Parents/Paper_Part.SocketLoc` _array_element) _inverse_2)
          (`KismetArrayLibrary.Array_RemoveItem` (`local.Links in`) _array_element)))))
  (if (> (`KismetArrayLibrary.Array_Length` _links_in) 0)
    (for _array_element_2 (`local.Links in`)
      ;[1 1 1] Gets the link out's name then attempts to socket to it.
      (bind _loc_2 (`self.Get Location Name` _array_element_2))
      (bind _inverse_3 (`self.InvertSocketName` _loc_2)) ; Link in name
      (bind _socketed (`self.SocketPart` _array_element_2 _inverse_3 self))
      (if _socketed
        (return true)
        (else
          (return false)))))
  (return false))

(fn `RotateSocketName`
  (params (Name :type Name) (Clockwise :type Boolean))
  (returns (New :type Name))
  (if Clockwise
    (switch `name` Name
      (:`South`
        (return "West"))
      (:`North`
        (return "East"))
      (:`West`
        (return "North"))
      (:`East`
        (return "South")))
    (else
      (switch `name` Name
        (:`South`
          (return "East"))
        (:`North`
          (return "East"))
        (:`West`
          (return "South"))
        (:`East`
          (return "North"))))))

(fn `SocketPart`
  (params (Loc :type Name) (Part :type "/Game/Tank/Blueprints/Parents/Paper_Part Object Reference"))
  (returns (Socketed :type Boolean))
  (locals (Var :type Integer))
  (bind _rendercomponent (`self.RenderComponent`))
  (bind _rootcomponent (`Actor.RootComponent` Part))
  (bind _returnvalue (`SceneComponent.GetAllSocketNames` _rendercomponent))
  (bind _output_get (set `/Game/Tank/Blueprints/Parents/Paper_Part.SocketLoc` Loc Part)) ; Remember which socket
  (switch `name` (`self.SocketLoc`)
    (:`Default`
      _)
    (:`South`
      _)
    (:`North`
      ;[1 1 1] Previous part was socketed to the north (therefore 180' rotaton). Socket to inverted requirement.
      (bind _inverse (`self.InvertSocketName` _output_get))
      (if (`KismetArrayLibrary.Array_Contains` _returnvalue _inverse)
        (bind _returnvalue_2 (`SceneComponent.K2_AttachToComponent` _rootcomponent _rendercomponent _inverse "SnapToTarget" "SnapToTarget" "KeepRelative" true)) ; Socket to prev part
        (return _returnvalue_2)
        (else
          (return false))))
    (:`West`
      ;[1 1 1] Previous part was socketed to the west (therefore a -90' rotation). Socket to Anticlockwise requirement.
      (bind _new (`self.RotateSocketName` _output_get))
      (if (`KismetArrayLibrary.Array_Contains` _returnvalue _new)
        (bind _returnvalue_3 (`SceneComponent.K2_AttachToComponent` _rootcomponent _rendercomponent _new "SnapToTarget" "SnapToTarget" "KeepRelative" true)) ; Socket to prev part
        (return _returnvalue_3)
        (else
          (return false))))
    (:`East`
      ;[1 1 1] Previous pat was socketed to the east (therefore a 90' rotation). Socket to clockwise requirement.
      (bind _new_2 (`self.RotateSocketName` _output_get true))
      (if (`KismetArrayLibrary.Array_Contains` _returnvalue _new_2)
        (bind _returnvalue_4 (`SceneComponent.K2_AttachToComponent` _rootcomponent _rendercomponent _new_2 "SnapToTarget" "SnapToTarget" "KeepRelative" true)) ; Socket to prev part
        (return _returnvalue_4)
        (else
          (return false)))))
  ;[1 1 1] Previous part was socketed to the south (therefore no rotation). Socket to required.
  (if (`KismetArrayLibrary.Array_Contains` _returnvalue _output_get)
    (bind _returnvalue_5 (`SceneComponent.K2_AttachToComponent` _rootcomponent _rendercomponent _output_get "SnapToTarget" "SnapToTarget" "KeepRelative" true)) ; Socket to prev part
    (return _returnvalue_5)
    (else
      (return false))))

(fn `UserConstructionScript`)