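; Parent Blueprint for a tank gun part that handles barrel aiming and firing.
; On BeginPlay it snaps GunBarrel to the GunSocket on RenderComponent.
; Aim flips barrel yaw for left or right facing, steps and clamps pitch by feeding world rotation into relative rotation, and prints the clamped angle.
; Fire spawns a half-scale ProjClass actor and an explosion emitter at the barrel's FireLoc socket.
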(event `self.ReceiveBeginPlay`
  (`SceneComponent.K2_AttachToComponent` (`self.GunBarrel`) (`self.RenderComponent`) "GunSocket" "SnapToTarget" "SnapToTarget" "KeepRelative" true))

(fn `Aim`
  (params (Aiming :type "Float (double-precision)") (IsRight :type Boolean))
  (bind _gunbarrel (`self.GunBarrel`))
  (bind _roll (.roll (`SceneComponent.K2_GetComponentRotation` _gunbarrel)))
  (bind _pitch (.pitch (`SceneComponent.K2_GetComponentRotation` _gunbarrel)))
  (bind _returnvalue (`KismetMathLibrary.FClamp` (.pitch (`SceneComponent.K2_GetComponentRotation` _gunbarrel)) -30.0 80.0))
  (if IsRight
    (`SceneComponent.K2_SetRelativeRotation` _gunbarrel (`KismetMathLibrary.MakeRotator` _roll _pitch 180.0) false false)
    (else
      (`SceneComponent.K2_SetRelativeRotation` _gunbarrel (`KismetMathLibrary.MakeRotator` _roll _pitch) false false)))
  (`SceneComponent.K2_AddLocalRotation` _gunbarrel (`KismetMathLibrary.MakeRotator` 0.0 (* Aiming -3.0)) false false)
  (`SceneComponent.K2_SetRelativeRotation` _gunbarrel (`KismetMathLibrary.MakeRotator` 0.0 _returnvalue (.yaw (`SceneComponent.K2_GetComponentRotation` _gunbarrel))) false false)
  (`KismetSystemLibrary.PrintString` (`KismetStringLibrary.Conv_DoubleToString` _returnvalue))
  (return))

(fn `Fire`
  (bind _gunbarrel (`self.GunBarrel`))
  (bind _returnvalue (`SceneComponent.GetSocketLocation` _gunbarrel "FireLoc"))
  (`|SpawnActorFromClass` (`self.ProjClass`) (`KismetMathLibrary.MakeTransform` _returnvalue (`SceneComponent.K2_GetComponentRotation` _gunbarrel) (0.5 0.5 0.5)) "Undefined" "OverrideRootScale" null null)
  (`GameplayStatics.SpawnEmitterAtLocation` "/Game/StarterContent/Particles/P_Explosion.P_Explosion" _returnvalue))

(fn `UserConstructionScript`
  (`parent.UserConstructionScript`))